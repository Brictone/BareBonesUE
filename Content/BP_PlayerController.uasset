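; Player controller that relays Enhanced Input movement actions to the possessed BP_Bare_Pawn.
; On BeginPlay it caches the controlled pawn, stopping if the cast fails, then adds the EIA_ActionMapping mapping context.
; The IA_Forward and IA_Right actions pass their values to the pawn's MoveForward and MoveSidways functions, leaving the movement logic to the pawn.
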(event Input|EnhancedActionEvents|EnhancedInputActionIA_Forward
  (params (ActionValue :type Float%20%28double-precision%29) (ElapsedSeconds :type Float%20%28double-precision%29) (TriggeredSeconds :type Float%20%28double-precision%29) (InputAction :type Input%20Action%20Object%20Reference :default "/Game/IA_Forward.IA_Forward"))
  (:Triggered
    (Default|MoveForward (Variables|Default|GetAs%20BP%20Bare%20Pawn) ActionValue)))

(event Input|EnhancedActionEvents|EnhancedInputActionIA_Right
  (params (ActionValue :type Float%20%28double-precision%29) (ElapsedSeconds :type Float%20%28double-precision%29) (TriggeredSeconds :type Float%20%28double-precision%29) (InputAction :type Input%20Action%20Object%20Reference :default "/Game/IA_Right.IA_Right"))
  (Default|MoveSidways (Variables|Default|GetAs%20BP%20Bare%20Pawn) ActionValue))

(event EventBeginPlay
  (bind _self self)
  (bind _returnvalue (PlayerController|LocalPlayerSubsystems|GetEnhancedInputLocalPlayerSubsystem _self))
  (bind _asbp_bare_pawn (Utilities|Casting|CastToBP_Bare_Pawn (Pawn|GetControlledPawn)))
  (Variables|Default|SetAs%20BP%20Bare%20Pawn _asbp_bare_pawn)
  (Utilities|IsValid _returnvalue
    (:Is%20Valid
      (Input|AddMappingContext _returnvalue "/Game/EIA_ActionMapping.EIA_ActionMapping" 0 "(bIgnoreAllPressedKeysUntilRelease=True,bForceImmediately=False,bNotifyUserSettings=False)"))))

(event EventTick
  (params (DeltaSeconds :type Float%20%28single-precision%29)))

(fn ConstructionScript)